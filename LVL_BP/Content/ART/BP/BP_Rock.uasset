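; BP_Rock procedurally builds a vertical stack of random meshes in its construction script; its variable names refer to books.
; A seeded stream picks each mesh, yaw, X/Z mirroring and scale, with scale also interpolated along the stack.
; Pieces are pitched 90 degrees and raised by accumulated, slightly shrunk bounding-box X widths.
; Width comes from separate random picks, so it may not match the placed mesh.
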(event EventBeginPlay)

(event Collision|EventActorBeginOverlap
  (params (OtherActor :type Actor%20Object%20Reference)))

(event EventTick
  (params (DeltaSeconds :type Float%20%28single-precision%29)))

(fn ConstructionScript
  (bind _randomrotation (Variables|Default|GetRandomRotation))
  (bind _nbrmesh (Variables|Default|GetNbrMesh))
  (Variables|Default|SetStream (Math|Random|MakeRandomStream (Variables|Default|GetInitialSeed)))
  ;[1 1 1] Loop
  (for _index (range 0 (- _nbrmesh 1))
    (Variables|Default|SetCurrent%20Random%20Scale (* (Math|Float|Lerp (Variables|Default|GetSize%20Scale%20Factor) 1.0 (/ _index _nbrmesh)) (Math|Random|RandomFloatinRangefromStream (Variables|Default|GetStream) (Variables|Default|GetRandom%20Factor%20Min) (Variables|Default|GetRandom%20Factor%20Max))))
    (Variables|Default|SetCurrentMesh (.OutItem (Utilities|Array|RandomFromStream (Variables|Default|GetMeshList) (Variables|Default|GetStream))))
    (bind _output_get (Variables|Default|SetCurrentBookWidth (* (* (- (.x (.max (StaticMesh|GetBoundingBox (.OutItem (Utilities|Array|RandomFromStream (Variables|Default|GetMeshList) (Variables|Default|GetStream)))))) (.x (.min (StaticMesh|GetBoundingBox (.OutItem (Utilities|Array|RandomFromStream (Variables|Default|GetMeshList) (Variables|Default|GetStream))))))) 0.9) (Variables|Default|GetCurrent%20Random%20Scale))))
    (bind _returnvalue (AddComponent|AddStaticMeshComponent false (Math|Transform|MakeTransform (Math|Vector|MakeVector 0.0 0.0 (+ (/ _output_get 2.0) (Variables|Default|GetTotalHeight))) (Math|Rotator|MakeRotator 0.0 9e+01 (Math|Random|RandomFloatinRangefromStream (Variables|Default|GetStream) (* _randomrotation -1.0) _randomrotation)) (* (Math|Vector|MakeVector (Math|Float|Lerp -1.0 1.0 (Math|Conversions|ToFloat(Boolean) (Math|Random|RandomBoolfromStream (Variables|Default|GetStream)))) 1.0 (Math|Float|Lerp -1.0 1.0 (Math|Conversions|ToFloat(Boolean) (Math|Random|RandomBoolfromStream (Variables|Default|GetStream))))) (Variables|Default|GetCurrent%20Random%20Scale)))))
    (bind _output_get_2 (Variables|Default|SetMesh _returnvalue))
    (Variables|Default|SetTotalHeight (+ (Variables|Default|GetTotalHeight) (Variables|Default|GetCurrentBookWidth)))
    (Components|StaticMesh|SetStaticMesh _output_get_2 (Variables|Default|GetCurrentMesh))))