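; BP_Random is an actor that shows a randomly picked static mesh, built entirely in its construction script.
; A random stream seeded by InitialSeed picks from MeshList, so the same seed and list give a repeatable result for an added mesh component.
; The mesh gets MI_FieldRadiusPreview on its first material slot.
; A seeded random unit vector is sent as a material parameter, but the parameter name is None.
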(event EventBeginPlay)

(event Collision|EventActorBeginOverlap
  (params (OtherActor :type Actor%20Object%20Reference)))

(event EventTick
  (params (DeltaSeconds :type Float%20%28single-precision%29)))

(fn ConstructionScript
  (Variables|Default|SetStream (Math|Random|MakeRandomStream (Variables|Default|GetInitial%20Seed)))
  (bind _returnvalue (AddComponent|AddStaticMeshComponent false))
  (bind _output_get (Variables|Default|SetStatic%20Mesh _returnvalue))
  (Components|StaticMesh|SetStaticMesh _output_get (.OutItem (Utilities|Array|RandomFromStream (Variables|Default|GetMesh%20List) (Variables|Default|GetStream))))
  (Rendering|Material|SetMaterial _output_get 0 "/Engine/EditorResources/FieldNodes/_Resources/MI_FieldRadiusPreview.MI_FieldRadiusPreview")
  (Rendering|Material|SetVectorParameterValueonMaterials (Variables|Default|GetStatic%20Mesh) "None" (Math|Random|RandomUnitVectorfromStream (Variables|Default|GetStream))))