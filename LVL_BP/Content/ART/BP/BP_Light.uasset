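; Lantern actor that can be configured as wall-mounted or floor-standing and switches on while something overlaps its Sphere component.
; Construction Script applies the IsOn state, then SetUpMesh shows either bracket or post and moves the lamp to the matching OnWall or OnFloor location.
; LightFunction drives the light's intensity, radius and color along with the lamp material's emissive parameters, turning it off again on end overlap.
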(event OnComponentBeginOverlap(Sphere)
  (params (OverlappedComponent :type Primitive%20Component%20Object%20Reference) (OtherActor :type Actor%20Object%20Reference) (OtherComp :type Primitive%20Component%20Object%20Reference) (OtherBodyIndex :type Integer) (bFromSweep :type Boolean) (SweepResult :type Hit%20Result%20Structure%20%28by%20ref%29))
  (CallFunction|LightFunction true))

(event OnComponentEndOverlap(Sphere)
  (params (OverlappedComponent :type Primitive%20Component%20Object%20Reference) (OtherActor :type Actor%20Object%20Reference) (OtherComp :type Primitive%20Component%20Object%20Reference) (OtherBodyIndex :type Integer))
  (CallFunction|LightFunction false))

(event EventBeginPlay)

(event Collision|EventActorBeginOverlap
  (params (OtherActor :type Actor%20Object%20Reference)))

(event EventTick
  (params (DeltaSeconds :type Float%20%28single-precision%29)))

(fn ConstructionScript
  (Utilities|FlowControl|Sequence
    (:then_0
      (CallFunction|LightFunction (Variables|Default|GetIs%20On)))
    (:then_1
      (CallFunction|SetUpMesh (Variables|Default|GetIsOnWall)))))

(fn LightFunction
  (params (Is%20On :type Boolean))
  (bind _lantern_light (Variables|Default|GetLantern_Light))
  (if Is%20On
    ;[1 1 1] Turn On
    (Rendering|Components|Light|SetIntensity _lantern_light (Variables|Default|GetIntensity))
    (Rendering|Lighting|SetAttenuationRadius _lantern_light (Variables|Default|GetRadius))
    (Rendering|Components|Light|SetLightColor _lantern_light (Variables|Default|GetLight%20Color) true)
    (Rendering|Material|SetVectorParameterValueonMaterials (Variables|Default|GetSM_Lamp) "Emissive Color" (Math|Conversions|ToVector(LinearColor) (Variables|Default|GetLight%20Color)))
    (Rendering|Material|SetScalarParameterValueonMaterials (Variables|Default|GetSM_Lamp) "Emissive Intensity" (/ (Variables|Default|GetIntensity) 1e+03))
    (else
      ;[1 1 1] Turn Off
      (Rendering|Components|Light|SetIntensity (Variables|Default|GetLantern_Light) 0.0)
      (Rendering|Material|SetScalarParameterValueonMaterials (Variables|Default|GetSM_Lamp) "Emissive Intensity" 0.0))))

(fn SetUpMesh
  (params (Is%20On :type Boolean))
  (if Is%20On
    ;[1 1 1] On Wall
    (Rendering|SetVisibility (Variables|Default|GetSM_Lamp_Post) false false)
    (Rendering|SetVisibility (Variables|Default|GetSM_Lamp_Bracket) true false)
    (Transformation|SetRelativeLocation (Variables|Default|GetSM_Lamp) (Variables|/Script/Engine.SceneComponent|GetRelativeLocation (Variables|Default|GetOn%20Wall)) false false)
    (else
      ;[1 1 1] On Floor
      (Rendering|SetVisibility (Variables|Default|GetSM_Lamp_Bracket) false false)
      (Rendering|SetVisibility (Variables|Default|GetSM_Lamp_Post) true false)
      (Transformation|SetRelativeLocation (Variables|Default|GetSM_Lamp) (Variables|/Script/Engine.SceneComponent|GetRelativeLocation (Variables|Default|GetOn%20Floor)) false false))))